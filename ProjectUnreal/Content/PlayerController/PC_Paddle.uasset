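; Player controller for a Breakout-style game that handles input for up to four paddles plus launching and restarting the ball.
; On BeginPlay it caches GM_BreakOut and the first paddle pawn and adds the Enhanced Input mapping context.
; Four move actions drive Player1 and the game mode's other paddles, but only while launched and not game over.
; Jump launches the ball, or after game over resets positions and restarts through the game mode.
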(event `self.ReceiveBeginPlay`
  (bind _asgm_break_out (cast `/Game/GameMods/GM_BreakOut` (`GameplayStatics.GetGameMode`)))
  (set `self.CurrentGameMode` _asgm_break_out)
  (`EnhancedInputSubsystemInterface.AddMappingContext` (subsystem `EnhancedInputLocalPlayerSubsystem`) "/Game/Inputs/IMC_Player.IMC_Player" 0 (struct))
  (bind _asbp_paddle_1 (cast `/Game/BluePrints/BP_Paddle1` (`GameplayStatics.GetPlayerPawn` 0)))
  (set `self.Player1` _asbp_paddle_1))

(event `EnhancedInput|/Game/Inputs/IA_Move1`
  (params (ActionValue :type "Float (double-precision)") (ElapsedSeconds :type "Float (double-precision)") (TriggeredSeconds :type "Float (double-precision)") (InputAction :type "InputAction Object Reference" :default "/Game/Inputs/IA_Move1.IA_Move1"))
  (:`Triggered`
    (if (`self.GameOver`)
      _
      (elif (`self.IsLaunched`)
        (`/Game/BluePrints/BP_Paddle1.Move` (`self.Player1`) ActionValue)))))

(event `EnhancedInput|/Game/Inputs/IA_Move2`
  (params (ActionValue :type "Float (double-precision)") (ElapsedSeconds :type "Float (double-precision)") (TriggeredSeconds :type "Float (double-precision)") (InputAction :type "InputAction Object Reference" :default "/Game/Inputs/IA_Move2.IA_Move2"))
  (:`Triggered`
    (if (`self.GameOver`)
      _
      (elif (`self.IsLaunched`)
        (`/Game/BluePrints/BP_Paddle2.Move` (`/Game/GameMods/GM_BreakOut.Player2` (`self.CurrentGameMode`)) ActionValue)))))

(event `EnhancedInput|/Game/Inputs/IA_Move3`
  (params (ActionValue :type "Float (double-precision)") (ElapsedSeconds :type "Float (double-precision)") (TriggeredSeconds :type "Float (double-precision)") (InputAction :type "InputAction Object Reference" :default "/Game/Inputs/IA_Move3.IA_Move3"))
  (:`Triggered`
    (if (`self.GameOver`)
      _
      (elif (`self.IsLaunched`)
        (`/Game/BluePrints/BP_Paddle3.Move` (`/Game/GameMods/GM_BreakOut.Player3` (`self.CurrentGameMode`)) ActionValue)))))

(event `EnhancedInput|/Game/Inputs/IA_Move4`
  (params (ActionValue :type "Float (double-precision)") (ElapsedSeconds :type "Float (double-precision)") (TriggeredSeconds :type "Float (double-precision)") (InputAction :type "InputAction Object Reference" :default "/Game/Inputs/IA_Move4.IA_Move4"))
  (:`Triggered`
    (if (`self.GameOver`)
      _
      (elif (`self.IsLaunched`)
        (`/Game/BluePrints/BP_Paddle4.Move` (`/Game/GameMods/GM_BreakOut.Player4` (`self.CurrentGameMode`)) ActionValue)))))

(event `EnhancedInput|/Game/Inputs/IA_Jump`
  (params (ActionValue :type "Float (double-precision)") (ElapsedSeconds :type "Float (double-precision)") (TriggeredSeconds :type "Float (double-precision)") (InputAction :type "InputAction Object Reference" :default "/Game/Inputs/IA_Jump.IA_Jump"))
  (bind _currentgamemode (`self.CurrentGameMode`))
  (bind _ball1 (`self.Ball1`))
  (bind _player1 (`self.Player1`))
  (:`Started`
    (if (`self.GameOver`)
      (set `self.IsLaunched` false)
      (set `self.GameOver` false)
      (`SceneComponent.K2_SetWorldLocation` (`/Game/BluePrints/BP_Ball1.Sphere` _ball1) (`/Game/BluePrints/BP_Ball1.StartPosition` _ball1) false false)
      (`SceneComponent.K2_SetWorldLocation` (`/Game/BluePrints/BP_Paddle1.Cube` _player1) (`/Game/BluePrints/BP_Paddle1.StartPosition` _player1) false false)
      (`/Game/GameMods/GM_BreakOut.RemoveWidgetGameOver` _currentgamemode)
      (`/Game/GameMods/GM_BreakOut.CreateWidgetLunchGame` _currentgamemode)
      (`/Game/GameMods/GM_BreakOut.RelunchGame` _currentgamemode)
      (elif (not (`self.IsLaunched`))
        (set `self.IsLaunched` true)
        (`/Game/GameMods/GM_BreakOut.LunchBall` (`self.CurrentGameMode`))
        (`/Game/GameMods/GM_BreakOut.RemoveWidgetLunchGame` (`self.CurrentGameMode`))))))

(fn `UserConstructionScript`)