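; BP_Paddle4 is a player paddle actor that slides horizontally along the world X axis.
; Its Move function takes an input value, scales it by MoveSpeed and frame delta time, and clamps the resulting X within fixed symmetric bounds, keeping Y and Z unchanged.
; BeginPlay caches the Cube component's world location as StartPosition, which is not read within this Blueprint.
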(event `self.ReceiveBeginPlay`
  (set `self.StartPosition` (`SceneComponent.K2_GetComponentLocation` (`self.Cube`))))

(fn `Move`
  (params (HorizontalMove :type "Float (double-precision)"))
  (locals (NewLocalVar :type "Actor Object Reference"))
  (bind (_returnvalue_x _returnvalue_y _returnvalue_z) (`KismetMathLibrary.BreakVector` (`self.K2_GetActorLocation`)))
  (`self.K2_SetActorLocation` (`KismetMathLibrary.MakeVector` (`KismetMathLibrary.FClamp` (+ _returnvalue_x (* HorizontalMove (`self.MoveSpeed`) (`GameplayStatics.GetWorldDeltaSeconds`))) -420.0 420.0) _returnvalue_y _returnvalue_z)))

(fn `UserConstructionScript`)