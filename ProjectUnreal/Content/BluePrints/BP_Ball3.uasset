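; Physics ball for a four-sided Breakout-style game with up to four paddles, launched along -X by the game mode's LunchBall event.
; Paddle hits call directional bounce functions that raise a speed multiplier and steer by the offset from the paddle, though Tick updates only Player 1's position.
; Hitting a game-over wall stops the ball and moves that side's closed wall into place; the game-over widget logic is unconnected.
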(event `self.ReceiveBeginPlay`
  (bind _asbp_paddle_1 (cast `/Game/BluePrints/BP_Paddle1` (`GameplayStatics.GetPlayerPawn` 0))
    (:`then`
      (set `self.Player1` _asbp_paddle_1)
      (bind _asgm_break_out (cast `/Game/GameMods/GM_BreakOut` (`GameplayStatics.GetGameMode`)))
      (set `self.Current Game Mode` _asgm_break_out)
      (set `self.StartPosition` (`SceneComponent.K2_GetComponentLocation` (`self.Sphere`)))
      (bind _aspc_paddle (cast `/Game/PlayerController/PC_Paddle` (`GameplayStatics.GetPlayerController` 0)))
      (set `self.CurrentPlayerController` _aspc_paddle)
      (add `/Game/GameMods/GM_BreakOut.LunchBallEvent` (`self.Current Game Mode`) (delegate `LunchBallEvent`)))
    (:`CastFailed`
      (bind _asbp_paddle_2 (cast `/Game/BluePrints/BP_Paddle2` (`GameplayStatics.GetPlayerPawn` 1))
        (:`then`
          (set `self.Player2` _asbp_paddle_2))
        (:`CastFailed`
          (bind _asbp_paddle_3 (cast `/Game/BluePrints/BP_Paddle3` (`GameplayStatics.GetPlayerPawn` 2))
            (:`then`
              (set `self.Player3` _asbp_paddle_3))
            (:`CastFailed`
              (bind _asbp_paddle_4 (cast `/Game/BluePrints/BP_Paddle4` (`GameplayStatics.GetPlayerPawn` 3)))
              (set `self.Player4` _asbp_paddle_4))))))))

(event `LunchBallEvent`
  (`self.LunchBalle`))

(event `self.ReceiveTick`
  (params (DeltaSeconds :type "Float (single-precision)"))
  (set `self.PlayerPosition1` (`self.K2_GetActorLocation` (`self.Player1`)))
  (set `self.MaxSpeed` (* (`self.MultiplicatorSpeed`) 94.0)))

(event `self.ReceiveHit`
  (params (MyComp :type "PrimitiveComponent Object Reference") (Other :type "Actor Object Reference") (OtherComp :type "PrimitiveComponent Object Reference") (bSelfMoved :type Boolean) (HitLocation :type "Vector Structure") (HitNormal :type "Vector Structure") (NormalImpulse :type "Vector Structure") (Hit :type "HitResult Structure (by ref)"))
  (cast `/Game/BluePrints/BP_Paddle1` Other
    (:`then`
      (`self.BounceUp`))
    (:`CastFailed`
      (cast `/Game/BluePrints/BP_Paddle2` Other
        (:`then`
          (`self.BounceRight`))
        (:`CastFailed`
          (cast `/Game/BluePrints/BP_Paddle3` Other
            (:`then`
              (`self.BounceDown`))
            (:`CastFailed`
              (cast `/Game/BluePrints/BP_Paddle4` Other
                (:`then`
                  (`self.BounceLeft`))
                (:`CastFailed`
                  (cast `/Game/BluePrints/BP_GameOverWall1` Other
                    (:`then`
                      (bind _returnvalue (`GameplayStatics.GetActorOfClass` "/Game/BluePrints/BP_WallClosed1.BP_WallClosed1_C"))
                      (`self.K2_SetActorLocation` _returnvalue (-500.0 0.0 0.0) false false))
                    (:`CastFailed`
                      (cast `/Game/BluePrints/BP_GameOverWall2` Other
                        (:`then`
                          (bind _returnvalue_2 (`GameplayStatics.GetActorOfClass` "/Game/BluePrints/BP_WallClosed2.BP_WallClosed2_C"))
                          (`self.K2_SetActorLocation` _returnvalue_2 (0.0 -500.0 0.0) false false))
                        (:`CastFailed`
                          (cast `/Game/BluePrints/BP_GameOverWall3` Other
                            (:`then`
                              (bind _returnvalue_3 (`GameplayStatics.GetActorOfClass` "/Game/BluePrints/BP_WallClosed3.BP_WallClosed3_C"))
                              (`self.K2_SetActorLocation` _returnvalue_3 (500.0 0.0 0.0) false false))
                            (:`CastFailed`
                              (cast `/Game/BluePrints/BP_GameOverWall4` Other)
                              (bind _returnvalue_4 (`GameplayStatics.GetActorOfClass` "/Game/BluePrints/BP_WallClosed4.BP_WallClosed4_C"))
                              (`self.K2_SetActorLocation` _returnvalue_4 (0.0 500.0 0.0) false false)))))))
                  (`PrimitiveComponent.SetPhysicsLinearVelocity` (`self.Sphere`) (0.0 0.0 0.0) false "None"))))))))))

(fn `BounceDown`
  (bind (_playerposition3_x _playerposition3_y) (`KismetMathLibrary.BreakVector` (`self.PlayerPosition3`)))
  (bind _maxspeed (`self.MaxSpeed`))
  (bind (_returnvalue_x _returnvalue_y) (`KismetMathLibrary.BreakVector` (`SceneComponent.K2_GetComponentLocation` (`self.Sphere`))))
  (bind _returnvalue (* (- _returnvalue_y _playerposition3_y) (`self.MultiplicatorSpeed`)))
  (bind _output_get (set `self.MultiplicatorSpeed` (+ (stale _output_get) 0.3)))
  (if (< _returnvalue 0.0)
    (`PrimitiveComponent.SetPhysicsLinearVelocity` (`self.Sphere`) (`KismetMathLibrary.MakeVector` (* (- _maxspeed (* _returnvalue -1.0)) -1.0) _returnvalue) false "None")
    (else
      (`PrimitiveComponent.SetPhysicsLinearVelocity` (`self.Sphere`) (`KismetMathLibrary.MakeVector` (* (- _maxspeed _returnvalue) -1.0) _returnvalue) false "None"))))

(fn `BounceLeft`
  (bind _playerposition4_x (`KismetMathLibrary.BreakVector` (`self.PlayerPosition4`)))
  (bind _maxspeed (`self.MaxSpeed`))
  (bind _returnvalue_x (`KismetMathLibrary.BreakVector` (`SceneComponent.K2_GetComponentLocation` (`self.Sphere`))))
  (bind _returnvalue (* (- _returnvalue_x _playerposition4_x) (`self.MultiplicatorSpeed`)))
  (bind _output_get (set `self.MultiplicatorSpeed` (+ (stale _output_get) 0.3)))
  (if (< _returnvalue 0.0)
    (`PrimitiveComponent.SetPhysicsLinearVelocity` (`self.Sphere`) (`KismetMathLibrary.MakeVector` _returnvalue (* (- _maxspeed (* _returnvalue -1.0)) -1.0)) false "None")
    (else
      (`PrimitiveComponent.SetPhysicsLinearVelocity` (`self.Sphere`) (`KismetMathLibrary.MakeVector` _returnvalue (* (- _maxspeed _returnvalue) -1.0)) false "None"))))

(fn `BounceRight`
  (bind _playerposition2_x (`KismetMathLibrary.BreakVector` (`self.PlayerPosition2`)))
  (bind _maxspeed (`self.MaxSpeed`))
  (bind _returnvalue_x (`KismetMathLibrary.BreakVector` (`SceneComponent.K2_GetComponentLocation` (`self.Sphere`))))
  (bind _returnvalue (* (- _returnvalue_x _playerposition2_x) (`self.MultiplicatorSpeed`)))
  (bind _output_get (set `self.MultiplicatorSpeed` (+ (stale _output_get) 0.3)))
  (if (< _returnvalue 0.0)
    (`PrimitiveComponent.SetPhysicsLinearVelocity` (`self.Sphere`) (`KismetMathLibrary.MakeVector` _returnvalue (- _maxspeed (* _returnvalue -1.0))) false "None")
    (else
      (`PrimitiveComponent.SetPhysicsLinearVelocity` (`self.Sphere`) (`KismetMathLibrary.MakeVector` _returnvalue (- _maxspeed _returnvalue)) false "None"))))

(fn `BounceUp`
  (bind _maxspeed (`self.MaxSpeed`))
  (bind (_playerposition1_x _playerposition1_y) (`KismetMathLibrary.BreakVector` (`self.PlayerPosition1`)))
  (bind (_returnvalue_x _returnvalue_y) (`KismetMathLibrary.BreakVector` (`SceneComponent.K2_GetComponentLocation` (`self.Sphere`))))
  (bind _returnvalue (* (- _returnvalue_y _playerposition1_y) (`self.MultiplicatorSpeed`)))
  (bind _output_get (set `self.MultiplicatorSpeed` (+ (stale _output_get) 0.3)))
  (if (< _returnvalue 0.0)
    (`PrimitiveComponent.SetPhysicsLinearVelocity` (`self.Sphere`) (`KismetMathLibrary.MakeVector` (- _maxspeed (* _returnvalue -1.0)) _returnvalue) false "None")
    (else
      (`PrimitiveComponent.SetPhysicsLinearVelocity` (`self.Sphere`) (`KismetMathLibrary.MakeVector` (- _maxspeed _returnvalue) _returnvalue) false "None"))))

(fn `LunchBalle`
  (`PrimitiveComponent.SetPhysicsLinearVelocity` (`self.Sphere`) (`KismetMathLibrary.MakeVector` (* (`self.MaxSpeed`) -1.0)) false "None"))

(fn `UserConstructionScript`)