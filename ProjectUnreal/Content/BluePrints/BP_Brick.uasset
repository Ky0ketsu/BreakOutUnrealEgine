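; Breakout brick actor that disappears with a Niagara effect when hit by BP_Ball1.
; Instead of being destroyed, the hit brick is moved 5000 units along X, out of its starting spot.
; On BeginPlay it stores the Cube's world position and binds to GM_BreakOut's restart event, which calls Replace to set the Cube back to that position.
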(event `self.ReceiveBeginPlay`
  (set `self.StartPosition` (`SceneComponent.K2_GetComponentLocation` (`self.Cube`)))
  (bind _asgm_break_out (cast `/Game/GameMods/GM_BreakOut` (`GameplayStatics.GetGameMode`)))
  (add `/Game/GameMods/GM_BreakOut.RestartGameEvent` _asgm_break_out (delegate `ReplaceBrickEvent`)))

(event `ReplaceBrickEvent`
  (`self.Replace`))

(event `self.ReceiveHit`
  (params (MyComp :type "PrimitiveComponent Object Reference") (Other :type "Actor Object Reference") (OtherComp :type "PrimitiveComponent Object Reference") (bSelfMoved :type Boolean) (HitLocation :type "Vector Structure") (HitNormal :type "Vector Structure") (NormalImpulse :type "Vector Structure") (Hit :type "HitResult Structure (by ref)"))
  (cast `/Game/BluePrints/BP_Ball1` Other)
  (`NiagaraFunctionLibrary.SpawnSystemAtLocation` "/Game/FX/NS_BrickDestroySysteme.NS_BrickDestroySysteme" (`SceneComponent.K2_GetComponentLocation` (`self.Cube`)))
  (`self.K2_SetActorLocation` (+ (`SceneComponent.K2_GetComponentLocation` (`self.Cube`)) (5000.0 0.0 0.0))))

(fn `Replace`
  (`SceneComponent.K2_SetWorldLocation` (`self.Cube`) (`self.StartPosition`) false false))

(fn `UserConstructionScript`)