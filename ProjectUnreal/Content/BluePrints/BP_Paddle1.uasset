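; BP_Paddle1 is a paddle actor that slides along the world Y axis within fixed limits.
; On BeginPlay it moves to the first PlayerStart found and stores its Cube's world location as StartPosition.
; Its Move function takes a horizontal value, scales it by MoveSpeed and delta seconds, and clamps the resulting Y while keeping X and Z.
; Tick and overlap events are empty, so movement relies on external calls to Move.
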(event `self.ReceiveBeginPlay`
  (bind _returnvalue (`GameplayStatics.GetActorOfClass` "/Script/Engine.PlayerStart"))
  (`self.K2_SetActorLocation` (`SceneComponent.K2_GetComponentLocation` (`Actor.RootComponent` _returnvalue)))
  (set `self.StartPosition` (`SceneComponent.K2_GetComponentLocation` (`self.Cube`))))

(fn `Move`
  (params (HorizontalMove :type "Float (double-precision)"))
  (locals (NewLocalVar :type "Actor Object Reference"))
  (bind (_returnvalue_x _returnvalue_y _returnvalue_z) (`KismetMathLibrary.BreakVector` (`self.K2_GetActorLocation`)))
  (`self.K2_SetActorLocation` (`KismetMathLibrary.MakeVector` _returnvalue_x (`KismetMathLibrary.FClamp` (+ _returnvalue_y (* HorizontalMove (`self.MoveSpeed`) (`GameplayStatics.GetWorldDeltaSeconds`))) -420.0 420.0) _returnvalue_z)))

(fn `UserConstructionScript`)