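; Game mode for a BreakOut game that spawns extra paddles and manages the launch and game over widgets.
; On BeginPlay it spawns paddles 2, 3 and 4 at fixed positions on three sides of the field, then shows the launch widget.
; Helper functions create or remove both widgets, while LunchBall and RelunchGame fire the ball launch and game restart events.
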(event `self.ReceiveBeginPlay`
  (`self.CreatePlayer`)
  (`self.CreateWidgetLunchGame`))

(fn `CreatePlayer`
  (bind _returnvalue (`|SpawnActorFromClass` "/Game/BluePrints/BP_Paddle2.BP_Paddle2_C" (`KismetMathLibrary.MakeTransform` (0.0 -1100.0 100.0) (struct :`Yaw` 90.0)) "DontSpawnIfColliding" "MultiplyWithRoot" null null))
  (set `self.Player2` _returnvalue)
  (bind _returnvalue_2 (`|SpawnActorFromClass` "/Game/BluePrints/BP_Paddle3.BP_Paddle3_C" (`KismetMathLibrary.MakeTransform` (1100.0 0.0 100.0) (struct :`Yaw` 180.0)) "DontSpawnIfColliding" "MultiplyWithRoot" null null))
  (set `self.Player3` _returnvalue_2)
  (bind _returnvalue_3 (`|SpawnActorFromClass` "/Game/BluePrints/BP_Paddle4.BP_Paddle4_C" (`KismetMathLibrary.MakeTransform` (0.0 1100.0 100.0) (struct :`Yaw` 90.0)) "DontSpawnIfColliding" "MultiplyWithRoot" null null))
  (set `self.Player4` _returnvalue_3))

(fn `CreateWidgetGameOver`
  (bind _returnvalue (`|CreateWidget` "/Game/Widget/WB_GameOver.WB_GameOver_C"))
  (bind _output_get (set `self.GameOverWidget` _returnvalue))
  (`UserWidget.AddToViewport` _output_get 0))

(fn `CreateWidgetLunchGame`
  (bind _returnvalue (`|CreateWidget` "/Game/Widget/WB_Lunch.WB_Lunch_C"))
  (bind _output_get (set `self.LunchBallWidget` _returnvalue))
  (`UserWidget.AddToViewport` _output_get 0))

(fn `LunchBall`
  (`self.LunchBallEvent`))

(fn `RelunchGame`
  (`self.RestartGameEvent`))

(fn `RemoveWidgetGameOver`
  (`Widget.RemoveFromParent` (`self.GameOverWidget`)))

(fn `RemoveWidgetLunchGame`
  (`Widget.RemoveFromParent` (`self.LunchBallWidget`)))

(fn `UserConstructionScript`)